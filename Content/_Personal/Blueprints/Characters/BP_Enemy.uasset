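; Patrolling enemy character that dies from any damage and can register itself with the player through a stealth-kill trigger.
; On BeginPlay it walks slowly through PatrolPoints via AIMoveTo, waiting after each successful arrival and looping to the first.
; Overlapping the trigger sets the player's NearbyEnemy to this enemy, and leaving clears it.
; Death turns the mesh into a ragdoll, disables capsule collision and sets IsDead, which makes Tick stop movement.
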(event OnComponentBeginOverlap(StealhKillTrigger)
  (params (OverlappedComponent :type Primitive%20Component%20Object%20Reference) (OtherActor :type Actor%20Object%20Reference) (OtherComp :type Primitive%20Component%20Object%20Reference) (OtherBodyIndex :type Integer) (bFromSweep :type Boolean) (SweepResult :type Hit%20Result%20Structure%20%28by%20ref%29))
  (bind _returnvalue (Game|GetPlayerCharacter 0))
  ;[0.15 0.15 0.15 0.5] Refactor SOON
  (if (== OtherActor _returnvalue)
    (bind _asbp_player (Utilities|Casting|CastToBP_Player _returnvalue))
    (Variables|/Game/_Personal/Blueprints/Characters/BP_Player.BP_Player_C|SetNearby%20Enemy _asbp_player self)))

(event OnComponentEndOverlap(StealhKillTrigger)
  (params (OverlappedComponent :type Primitive%20Component%20Object%20Reference) (OtherActor :type Actor%20Object%20Reference) (OtherComp :type Primitive%20Component%20Object%20Reference) (OtherBodyIndex :type Integer))
  (bind _returnvalue (Game|GetPlayerCharacter 0))
  ;[0.15 0.15 0.15 0.5] Refactor SOON
  (if (== OtherActor _returnvalue)
    (bind _asbp_player (Utilities|Casting|CastToBP_Player _returnvalue))
    (Variables|/Game/_Personal/Blueprints/Characters/BP_Player.BP_Player_C|SetNearby%20Enemy _asbp_player 0)))

(event EventTick
  (params (DeltaSeconds :type Float%20%28single-precision%29))
  ;[0.15 0.15 0.15 0.5] Refactor SOON
  (if (Variables|Default|GetIs%20Dead?)
    (Class|NavMovementInterface|StopActiveMovement (Variables|Character|GetCharacterMovement))))

(event Game|Damage|EventAnyDamage
  (params (Damage :type Float%20%28single-precision%29) (DamageType :type Damage%20Type%20Object%20Reference) (InstigatedBy :type Controller%20Object%20Reference) (DamageCauser :type Actor%20Object%20Reference))
  ;[0.15 0.15 0.15 0.5] Refactor SOON
  (CallFunction|Death))

(event EventBeginPlay
  ;[0.15 0.15 0.15 0.5] Refactor SOON
  (Variables|/Script/Engine.CharacterMovementComponent|SetMaxWalkSpeed (Variables|Character|GetCharacterMovement) 1.5e+02)
  (if (not (<= (Utilities|Array|Length (Variables|Default|GetPatrol%20Points)) 0))
    (AI|AIMoveTo self "0, 0, 0" (Utilities|Array|Get(acopy) (Variables|Default|GetPatrol%20Points) (Variables|Default|GetCurrent%20Patrol%20Point%20Index)) 5e+01 false :!label _label
      (:OnSuccess
        (Utilities|FlowControl|Delay (Variables|Default|GetWait%20Time%20per%20Patrol%20Point))
        (bind _result (Math|Integer|IncrementInt (Variables|Default|GetCurrent%20Patrol%20Point%20Index))
          (:%20%20
            (if (>= _result (Utilities|Array|Length (Variables|Default|GetPatrol%20Points)))
              (Variables|Default|SetCurrent%20Patrol%20Point%20Index 0)
              (goto _label)
              (else
                (goto _label)))))))))

(fn ConstructionScript)

(fn Death
  (Physics|SetSimulatePhysics (Variables|Character|GetMesh) true)
  (Class|SkeletalMeshComponent|SetPhysicsBlendWeight (Variables|Character|GetMesh) 1.0)
  (Collision|SetCollisionEnabled (Variables|Character|GetMesh) "QueryAndPhysics")
  (Collision|SetCollisionEnabled (Variables|Collision|GetCapsuleComponent) "NoCollision")
  (Variables|Default|SetIs%20Dead? true))