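; NPC character that reacts to being damaged with dialogue and can ragdoll on death.
; Any damage picks a random entry from FriendlyFireDialogues and shows it, with no health tracking or dead-state check.
; A separate Death function, not called within this Blueprint, enables mesh physics, disables capsule collision and sets IsDead.
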(event Game|Damage|EventAnyDamage
  (params (Damage :type Float%20%28single-precision%29) (DamageType :type Damage%20Type%20Object%20Reference) (InstigatedBy :type Controller%20Object%20Reference) (DamageCauser :type Actor%20Object%20Reference))
  (bind _friendly_fire_dialogues (Variables|Default|GetFriendly%20Fire%20Dialogues))
  ;[0.15 0.15 0.15 0.5] Refactor SOON
  (Default|ShowDialogueEvent (Utilities|Array|Get(acopy) _friendly_fire_dialogues (Math|Random|RandomInteger (Utilities|Array|Length _friendly_fire_dialogues)))))

(fn ConstructionScript)

(fn Death
  (Physics|SetSimulatePhysics (Variables|Character|GetMesh) true)
  (Class|SkeletalMeshComponent|SetPhysicsBlendWeight (Variables|Character|GetMesh) 1.0)
  (Collision|SetCollisionEnabled (Variables|Character|GetMesh) "QueryAndPhysics")
  (Collision|SetCollisionEnabled (Variables|Collision|GetCapsuleComponent) "NoCollision")
  (Variables|Default|SetIs%20Dead? true))