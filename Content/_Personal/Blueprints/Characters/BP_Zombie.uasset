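; BP_Zombie is a zombie character Blueprint that can be shown or hidden as part of a numbered batch.
; BatchCall compares the instance's BatchNumber to an activate ID and a deactivate ID, unhiding on the first match or hiding and disabling collision on the second.
; Activation does not re-enable collision, and the function is flagged for refactoring.
; BeginPlay, Tick and the construction script add no logic of their own.
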(event EventBeginPlay)

(event EventTick
  (params (DeltaSeconds :type Float%20%28single-precision%29))
  (|CallParentFunction DeltaSeconds) ; This node is disabled and will not be called.\nDrag off pins to build functionality.
)

(fn ConstructionScript
  (|CallParentFunction))

(fn BatchCall
  (params (Batch%20ID%20to%20Activate :type Integer) (Batch%20ID%20to%20Deactivate :type Integer))
  ;[0.15 0.15 0.15 0.5] Refactor SOON
  (if (== Batch%20ID%20to%20Activate (Variables|Default|GetBatch%20Number))
    (Rendering|SetActorHiddenInGame false)
    (elif (== Batch%20ID%20to%20Deactivate (Variables|Default|GetBatch%20Number))
      (Rendering|SetActorHiddenInGame true)
      (Collision|SetActorEnableCollision false))))