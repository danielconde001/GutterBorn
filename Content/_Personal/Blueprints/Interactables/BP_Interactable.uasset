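; BP_Interactable is a generic interactable with Interact and Stop Interacting functions, apparently meant as a base for interactable objects.
; On BeginPlay it finds the BP_Player actor with GetActorOfClass and caches it in Player.
; Both functions only print a debug message with the object's display name, and the construction script is empty.
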(event EventBeginPlay
  (bind _returnvalue (Actor|GetActorOfClass "/Game/_Personal/Blueprints/Characters/BP_Player.BP_Player_C"))
  (Variables|Default|SetPlayer _returnvalue))

(fn ConstructionScript)

(fn Interact
  (Development|PrintString (Utilities|String|Append "Interacting with " (Utilities|GetDisplayName self))))

(fn StopInteracting
  (Development|PrintString (Utilities|String|Append "Stopped interacting with " (Utilities|GetDisplayName self))))