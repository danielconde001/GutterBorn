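; Interactable that lets the player boost an assigned NPC, moving it instantly to a boost location actor with a sound effect.
; Trigger overlaps set or clear it as the player's nearby interactable, and Interact runs the boost, subject to availability and optional one-time-use checks.
; The boost calls NPCDoesSomething on the BP_NPC, records completion, and toggles visibility and collision on lists of actors to disable and enable.
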(event OnComponentBeginOverlap(Trigger)
  (params (OverlappedComponent :type Primitive%20Component%20Object%20Reference) (OtherActor :type Actor%20Object%20Reference) (OtherComp :type Primitive%20Component%20Object%20Reference) (OtherBodyIndex :type Integer) (bFromSweep :type Boolean) (SweepResult :type Hit%20Result%20Structure%20%28by%20ref%29))
  (CallFunction|SetNearbyInteractableforPlayer OtherActor self))

(event OnComponentEndOverlap(Trigger)
  (params (OverlappedComponent :type Primitive%20Component%20Object%20Reference) (OtherActor :type Actor%20Object%20Reference) (OtherComp :type Primitive%20Component%20Object%20Reference) (OtherBodyIndex :type Integer))
  (CallFunction|SetNearbyInteractableforPlayer OtherActor))

(event Custom|Boost%20NPC%20On%20Interact
  (if (Variables|Default|GetCan%20be%20interacted%20with?)
    (if (Variables|Default|GetCan%20be%20interacted%20with%20only%20once?)
      (if (not (Variables|Default|GetHas%20been%20interacted%20with%20already?))
        (Audio|PlaySoundatLocation "/Game/_Personal/Audio/SFX_NPCBoost.SFX_NPCBoost" (Transformation|GetActorLocation) "0, 0, 0" 1.0 1.0 0.0 0 0 0 0 :!label _label)
        (Transformation|SetActorLocation (Variables|Default|GetNPC%20to%20Boost) (Transformation|GetActorLocation (Variables|Default|GetBoost%20Location)) false false)
        (bind _asbp_npc (Utilities|Casting|CastToBP_NPC (Variables|Default|GetNPC%20to%20Boost)))
        (Default|NPCDoesSomething _asbp_npc)
        (Variables|Default|SetBoost%20has%20been%20done? true)
        (Variables|Default|SetHas%20been%20interacted%20with%20already? true)
        (CallFunction|Disable/EnableActors))
      (else
        (goto _label)))))

(event Custom|Disable/Enable%20Actors
  ;[0.15 0.15 0.15 0.5] Refactor this trash code eventually, use Event Dispatchers
  (for _array_element (Variables|Default|GetActors%20to%20Disable%20on%20Interact)
    (Rendering|SetActorHiddenInGame _array_element true)
    (Collision|SetActorEnableCollision _array_element false))
  (for _array_element_2 (Variables|Default|GetActors%20to%20Enable%20on%20Interact)
    (Rendering|SetActorHiddenInGame _array_element_2 false)
    (Collision|SetActorEnableCollision _array_element_2 true)))

(event EventBeginPlay
  (|CallParentFunction) ; This node is disabled and will not be called.\nDrag off pins to build functionality.
)

(fn ConstructionScript
  (|CallParentFunction))

(fn Interact
  (|CallParentFunction)
  (CallFunction|BoostNPConInteract))