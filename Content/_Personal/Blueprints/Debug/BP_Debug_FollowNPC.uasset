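; Debug waypoint actor that shows optional text and advances a chained sequence when the player walks into its box.
; While activated, an overlap by player character 0 reveals ActorsToEnable with collision and hides ActorsToDisable without it.
; Enabled BP_Debug_FollowNPC and BP_Debug_Teleporter actors are set activated, so each step arms the next.
; The actor then hides itself and disables its collision.
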(event OnComponentBeginOverlap(Box)
  (params (OverlappedComponent :type Primitive%20Component%20Object%20Reference) (OtherActor :type Actor%20Object%20Reference) (OtherComp :type Primitive%20Component%20Object%20Reference) (OtherBodyIndex :type Integer) (bFromSweep :type Boolean) (SweepResult :type Hit%20Result%20Structure%20%28by%20ref%29))
  (bind _self self)
  (if (== (Game|GetPlayerCharacter 0) OtherActor)
    (if (Variables|DebugSettings|GetIs%20Activated?)
      (for _array_element (Variables|DebugSettings|GetActors%20to%20Enable)
        (Utilities|IsValid _array_element
          (:Is%20Valid
            (Rendering|SetActorHiddenInGame _array_element false)
            (Collision|SetActorEnableCollision _array_element true)
            (bind _asbp_debug_follow_npc (Utilities|Casting|CastToBP_Debug_FollowNPC _array_element)
              (:then
                (Variables|BP_Debug_FollowNPC_C|SetIs%20Activated? _asbp_debug_follow_npc true))
              (:CastFailed
                (bind _asbp_debug_teleporter (Utilities|Casting|CastToBP_Debug_Teleporter _array_element))
                (Variables|/Game/_Personal/Blueprints/Debug/BP_Debug_Teleporter.BP_Debug_Teleporter_C|SetIs%20Activated? _asbp_debug_teleporter true))))))
      (for _array_element_2 (Variables|DebugSettings|GetActors%20to%20Disable)
        (Utilities|IsValid _array_element_2
          (:Is%20Valid
            (Rendering|SetActorHiddenInGame _array_element_2 true)
            (Collision|SetActorEnableCollision _array_element_2 false))))
      (Rendering|SetActorHiddenInGame _self true)
      (Collision|SetActorEnableCollision _self false))))

(event EventBeginPlay
  (if (Variables|DebugSettings|GetText%20String%20is%20Empty?)
    (Rendering|Components|TextRender|SetText (Variables|Default|GetTextRender) (Class|KismetTextLibrary|GetEmptyText))
    (else
      (Rendering|Components|TextRender|SetText (Variables|Default|GetTextRender) (Utilities|Text|ToText(String) (Variables|DebugSettings|GetText%20String))))))

(fn ConstructionScript)