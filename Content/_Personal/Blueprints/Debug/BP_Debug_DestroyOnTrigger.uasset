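; Debug trigger volume that destroys an assigned actor when the player character overlaps its box.
; After a configurable delay it stops the player's movement, disables input, and destroys the target actor.
; One second later it re-enables input and destroys itself, making it a one-shot trigger.
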(event OnComponentBeginOverlap(Box)
  (params (OverlappedComponent :type Primitive%20Component%20Object%20Reference) (OtherActor :type Actor%20Object%20Reference) (OtherComp :type Primitive%20Component%20Object%20Reference) (OtherBodyIndex :type Integer) (bFromSweep :type Boolean) (SweepResult :type Hit%20Result%20Structure%20%28by%20ref%29))
  (bind _returnvalue (Game|GetPlayerCharacter 0))
  (if (== OtherActor _returnvalue)
    (Utilities|FlowControl|Delay (Variables|Default|GetDelay))
    (Components|Movement|StopMovementImmediately (Variables|/Script/Engine.Character|GetCharacterMovement _returnvalue))
    (Input|DisableInput (Game|Player|GetPlayerPawn 0) (Game|GetPlayerController 0))
    (Actor|DestroyActor (Variables|Default|GetActor%20To%20Destroy))
    (Utilities|FlowControl|Delay 1.0)
    (Input|EnableInput (Game|Player|GetPlayerPawn 0) (Game|GetPlayerController 0))
    (Actor|DestroyActor)))

(fn ConstructionScript)