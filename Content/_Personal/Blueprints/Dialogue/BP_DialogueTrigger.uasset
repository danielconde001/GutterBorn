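; Dialogue trigger actor that shows timed, colored dialogue lines on screen, started by ShowDialogueEvent or optionally by the player entering its trigger volume.
; It registers with BP_DialogueManager, either interrupting the current dialogue or starting only when none is playing.
; A Delay-driven loop steps parallel text, color and duration arrays through a W_DialogueUI widget.
; When lines run out or another dialogue takes over, it removes the widget and notifies the manager.
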(event OnComponentBeginOverlap(Trigger)
  (params (OverlappedComponent :type Primitive%20Component%20Object%20Reference) (OtherActor :type Actor%20Object%20Reference) (OtherComp :type Primitive%20Component%20Object%20Reference) (OtherBodyIndex :type Integer) (bFromSweep :type Boolean) (SweepResult :type Hit%20Result%20Structure%20%28by%20ref%29))
  (if (Variables|Default|GetUses%20Trigger%20Volume?)
    (if (== OtherActor (Game|GetPlayerCharacter 0))
      (CallFunction|ShowDialogueEvent))))

(event Custom|Show%20Dialogue%20Event
  (if (Variables|Default|GetCan%20Interrupt%20Current%20Dialogue?)
    (Default|RemoveCurrentDialogue (Variables|Default|GetDialogue%20Manager))
    (if (not (Variables|Default|GetIs%20Currently%20Playing?)) :!label _label
      (if (Variables|Default|GetPlay%20Only%20Once?)
        (Utilities|FlowControl|DoOnce false
          (:Completed
            _)))
      (Variables|/Game/_Personal/Blueprints/Dialogue/BP_DialogueManager.BP_DialogueManager_C|SetCurrent%20Dialogue (Variables|Default|GetDialogue%20Manager) self)
      (bind _returnvalue (UserInterface|CreateWidget "/Game/_Personal/Blueprints/Widgets/W_DialogueUI.W_DialogueUI_C" (Game|GetPlayerController 0)))
      (bind _output_get (Variables|Default|SetCurrent%20Dialogue%20Widget _returnvalue))
      (Variables|Default|SetIs%20Currently%20Playing? true)
      (Variables|Default|SetCurrent%20Dialogue%20Index 0)
      (if (and (< (Variables|Default|GetCurrent%20Dialogue%20Index) (Utilities|Array|Length (Variables|Default|GetDialogue%20To%20Say))) (== (Variables|/Game/_Personal/Blueprints/Dialogue/BP_DialogueManager.BP_DialogueManager_C|GetCurrent%20Dialogue (Variables|Default|GetDialogue%20Manager)) self)) :!label _label_2
        (Rendering|Components|TextRender|SetText (Variables|/Game/_Personal/Blueprints/Widgets/W_DialogueUI.W_DialogueUI_C|GetDialogueText _output_get) (Utilities|Text|ToText(String) (Utilities|Array|Get(acopy) (Variables|Default|GetDialogue%20To%20Say) (Variables|Default|GetCurrent%20Dialogue%20Index))))
        (Appearance|SetColorandOpacity _output_get (Math|Conversions|ToLinearColor(Color) (Utilities|Array|Get(acopy) (Variables|Default|GetDialogue%20Color) (Variables|Default|GetCurrent%20Dialogue%20Index))) :!class /Script/UMG.UserWidget)
        (UserInterface|Viewport|AddtoViewport _output_get 0)
        (Utilities|FlowControl|Delay (Utilities|Array|Get(acopy) (Variables|Default|GetDelay%20Timer) (Variables|Default|GetCurrent%20Dialogue%20Index)))
        (Math|Integer|IncrementInt (Variables|Default|GetCurrent%20Dialogue%20Index)
          (:%20%20
            (goto _label_2)))
        (else
          (Widget|RemovefromParent _output_get)
          (Variables|Default|SetIs%20Currently%20Playing? false)
          (Default|OnDialogueEnd (Variables|Default|GetDialogue%20Manager) self))))
    (else
      (bind _bool_value (Default|IsADialogueCurrentlyPlaying? (Variables|Default|GetDialogue%20Manager)))
      (if (not _bool_value)
        (goto _label)))))

(event EventBeginPlay
  (bind _returnvalue (Actor|GetActorOfClass "/Game/_Personal/Blueprints/Dialogue/BP_DialogueManager.BP_DialogueManager_C"))
  (Variables|Default|SetDialogue%20Manager _returnvalue)
  (if (Variables|Default|GetDisable%20Collision%20On%20BeginPlay?)
    (Collision|SetActorEnableCollision false)))

(fn ConstructionScript)