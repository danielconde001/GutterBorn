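; BP_BreakableLock is a shootable lock that breaks when shot and can unlock a linked set of double doors.
; It extends the parent's shot reaction by calling OnShotReaction, which clears IsLocked if the LinkedInteractable casts to BPI_DoubleDoors.
; When CallsInteractOnShot is set, it also calls Interact on the linked object, then the lock destroys itself.
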(event Custom|On%20Shot%20Reaction
  (bind _asbp_small_gate (Utilities|Casting|CastToBPI_DoubleDoors (Variables|Default|GetLinked%20Interactable))
    (:then
      (Variables|/Game/_Personal/Blueprints/Interactables/BPI_DoubleDoors.BPI_DoubleDoors_C|SetIs%20Locked? _asbp_small_gate false))
    (:CastFailed
      _))
  (if (Variables|Default|GetCalls%20Interact%20On%20Shot?)
    (Default|Interact (Variables|Default|GetLinked%20Interactable)))
  (Actor|DestroyActor))

(fn ConstructionScript
  (|CallParentFunction))

(fn ReactionwhenShotat
  (|CallParentFunction)
  (CallFunction|OnShotReaction))