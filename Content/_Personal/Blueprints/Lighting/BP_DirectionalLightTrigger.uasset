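; Trigger volume that blends the level's directional light between indoor and outdoor settings as the player enters or leaves its box.
; BeginPlay caches the first DirectionalLight actor found in the level.
; Player overlap begin plays an indoors timeline and overlap end plays an outdoors timeline, each driving the light component's shadow amount and intensity.
; The two transitions are separate forward-played timelines rather than one reversed.
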(event OnComponentBeginOverlap(Box)
  (params (OverlappedComponent :type Primitive%20Component%20Object%20Reference) (OtherActor :type Actor%20Object%20Reference) (OtherComp :type Primitive%20Component%20Object%20Reference) (OtherBodyIndex :type Integer) (bFromSweep :type Boolean) (SweepResult :type Hit%20Result%20Structure%20%28by%20ref%29))
  (bind _directional_light (Variables|Default|GetDirectional%20Light))
  (bind _returnvalue (Actor|GetComponentbyClass _directional_light "/Script/Engine.DirectionalLightComponent"))
  (if (== OtherActor (Game|GetPlayerCharacter 0))
    (bind (_direction _shadow_amount _intensity) (Timeline|Indoors%20Timeline Play)
      (:Update
        (Utilities|FlowControl|Sequence
          (:then_0
            (Class|DirectionalLightComponent|SetShadowAmount _returnvalue _shadow_amount))
          (:then_1
            (Rendering|Components|Light|SetIntensity _returnvalue _intensity)))))))

(event OnComponentEndOverlap(Box)
  (params (OverlappedComponent :type Primitive%20Component%20Object%20Reference) (OtherActor :type Actor%20Object%20Reference) (OtherComp :type Primitive%20Component%20Object%20Reference) (OtherBodyIndex :type Integer))
  (bind _directional_light (Variables|Default|GetDirectional%20Light))
  (bind _returnvalue (Actor|GetComponentbyClass _directional_light "/Script/Engine.DirectionalLightComponent"))
  (if (== OtherActor (Game|GetPlayerCharacter 0))
    (bind (_direction _shadow_amount _intensity) (Timeline|Outdoors%20Timeline Play)
      (:Update
        (Utilities|FlowControl|Sequence
          (:then_0
            (Class|DirectionalLightComponent|SetShadowAmount _returnvalue _shadow_amount))
          (:then_1
            (Rendering|Components|Light|SetIntensity _returnvalue _intensity)))))))

(event EventBeginPlay
  (bind _returnvalue (Actor|GetActorOfClass "/Script/Engine.DirectionalLight"))
  (Variables|Default|SetDirectional%20Light _returnvalue))

(fn ConstructionScript)