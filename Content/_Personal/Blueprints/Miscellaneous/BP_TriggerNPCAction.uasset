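; BP_TriggerNPCAction is a placeable trigger that tells a referenced NPC to perform an action identified by an ActionID.
; The TriggerNPCAction event calls NPCDoesAction on that NPC and can be invoked directly.
; When UseTriggerVolume is enabled, the player character overlapping the Box also fires it, guarded by a flag so the overlap path runs only once.
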(event OnComponentBeginOverlap(Box)
  (params (OverlappedComponent :type Primitive%20Component%20Object%20Reference) (OtherActor :type Actor%20Object%20Reference) (OtherComp :type Primitive%20Component%20Object%20Reference) (OtherBodyIndex :type Integer) (bFromSweep :type Boolean) (SweepResult :type Hit%20Result%20Structure%20%28by%20ref%29))
  (if (Variables|Default|GetUse%20Trigger%20Volume?)
    (if (== OtherActor (Game|GetPlayerCharacter 0))
      (if (not (Variables|Default|GetHas%20been%20interacted%20with%20already?))
        (CallFunction|TriggerNPCAction)
        (Variables|Default|SetHas%20been%20interacted%20with%20already? true)))))

(event Custom|Trigger%20NPC%20Action
  (Default|NPCDoesAction (Variables|Default|GetNPC) (Variables|Default|GetAction%20ID)))

(fn ConstructionScript)