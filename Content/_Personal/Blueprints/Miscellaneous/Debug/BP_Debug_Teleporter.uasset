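; BP_Debug_Teleporter is a debug actor that moves the player to the location of a target actor.
; On BeginPlay it sets its text render label to the configured string, or blanks it when flagged empty.
; When the first player character overlaps its box while the teleporter is activated, it sets that character's location to GoToActor's, without sweep and leaving rotation untouched.
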(event OnComponentBeginOverlap(Box)
  (params (OverlappedComponent :type Primitive%20Component%20Object%20Reference) (OtherActor :type Actor%20Object%20Reference) (OtherComp :type Primitive%20Component%20Object%20Reference) (OtherBodyIndex :type Integer) (bFromSweep :type Boolean) (SweepResult :type Hit%20Result%20Structure%20%28by%20ref%29))
  (if (== (Game|GetPlayerCharacter 0) OtherActor)
    (if (Variables|DebugTeleporter|GetIs%20Activated?)
      (Transformation|SetActorLocation OtherActor (Transformation|GetActorLocation (Variables|DebugTeleporter|GetGo%20To%20Actor)) false false))))

(event EventBeginPlay
  (if (Variables|DebugTeleporter|GetText%20String%20is%20Empty?)
    (Rendering|Components|TextRender|SetText (Variables|Default|GetTextRender) (Class|KismetTextLibrary|GetEmptyText))
    (else
      (Rendering|Components|TextRender|SetText (Variables|Default|GetTextRender) (Utilities|Text|ToText(String) (Variables|DebugTeleporter|GetText%20String))))))

(fn ConstructionScript)