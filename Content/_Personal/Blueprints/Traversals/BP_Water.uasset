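; BP_Water is a water volume actor that switches the player's swimming state as they enter and leave its mesh.
; Mesh overlap events set a per-volume HasPlayerInIt flag and call StartSwimming on BP_Player when entering.
; On exit it asks the BP_WaterManager found at BeginPlay whether the player is still in water, calling StopSwimming only if not.
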(event OnComponentBeginOverlap(Mesh)
  (params (OverlappedComponent :type Primitive%20Component%20Object%20Reference) (OtherActor :type Actor%20Object%20Reference) (OtherComp :type Primitive%20Component%20Object%20Reference) (OtherBodyIndex :type Integer) (bFromSweep :type Boolean) (SweepResult :type Hit%20Result%20Structure%20%28by%20ref%29))
  (bind _returnvalue (Game|GetPlayerCharacter 0))
  (if (== OtherActor _returnvalue)
    (Variables|Default|SetHas%20Player%20in%20it? true)
    (bind _asbp_player (Utilities|Casting|CastToBP_Player _returnvalue))
    (Default|StartSwimming _asbp_player)))

(event OnComponentEndOverlap(Mesh)
  (params (OverlappedComponent :type Primitive%20Component%20Object%20Reference) (OtherActor :type Actor%20Object%20Reference) (OtherComp :type Primitive%20Component%20Object%20Reference) (OtherBodyIndex :type Integer))
  (bind _returnvalue (Game|GetPlayerCharacter 0))
  (if (== OtherActor _returnvalue)
    (Variables|Default|SetHas%20Player%20in%20it? false)
    (bind _asbp_player (Utilities|Casting|CastToBP_Player _returnvalue))
    (bind _value (Default|IsPlayerStillinWater? (Variables|Default|GetWater%20Manager)))
    (if (not _value)
      (Default|StopSwimming _asbp_player))))

(event EventBeginPlay
  (bind _returnvalue (Actor|GetActorOfClass "/Game/_Personal/Blueprints/Traversals/BP_WaterManager.BP_WaterManager_C"))
  (Variables|Default|SetWater%20Manager _returnvalue))

(fn ConstructionScript)